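; Function library with ModN, a modulo that wraps a number into a ring, noted as the basis for all cyclic parameter changes in the project.
; ModN recursively adds or subtracts LastRingNum for values outside the range from FirstRingNum up to, but excluding, LastRingNum.
; The step is LastRingNum rather than the range width, so results can land outside the range when FirstRingNum is nonzero.
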(fn ModN
  (params (Value :type Integer) (First_Ring_Num :type Integer) (Last_Ring_Num :type Integer))
  (bind _returnvalue (- Value Last_Ring_Num))
  (bind _returnvalue_2 (+ Value Last_Ring_Num))
  ;[1 0.25 1] Очень важная для данного проекта математическая функиция, реализующая модуль над некоторым кольцом чисел. Это функция основа всех цикличиских смен параметров в этом проекте.
  (if (< Value First_Ring_Num)
    (if (< _returnvalue_2 First_Ring_Num)
      (bind _return_value (CallFunction|ModN _returnvalue_2 First_Ring_Num Last_Ring_Num))
      (return _return_value)
      (else
        (return _returnvalue_2)))
    (elif (>= Value Last_Ring_Num)
      (if (>= _returnvalue Last_Ring_Num)
        (bind _return_value_2 (CallFunction|ModN _returnvalue First_Ring_Num Last_Ring_Num))
        (return _return_value_2)
        (elif (< _returnvalue First_Ring_Num)
          (bind _return_value_3 (CallFunction|ModN _returnvalue First_Ring_Num Last_Ring_Num))
          (return _return_value_3)
          (else
            (return _returnvalue))))
      (else
        (return Value)))))