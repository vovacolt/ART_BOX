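; C_ART_BOX_BP is a manager that configures and starts every A_Art_Widget actor in the level.
; On BeginPlay or Init, it sends a count request through VUDBComp, then gives each widget its index, the widget total as update period, a staggered start delay and a random delay between artworks before initializing it.
; The failed-request branch that would break the socket connection and notify A_GameMenu is unwired.
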(event Custom|Init
  (bind _returnvalue (Class|CMARTBOXDB|FonCountReq (Variables|Default|GetvUDBComp)))
  (bind _outactors (Actor|GetAllActorsOfClass "/Game/Code/Blueprints/Widget/A_Art_Widget.A_Art_Widget_C"))
  (for (_array_element _array_index) _outactors
    (Utilities|FlowControl|Sequence
      (:then_0
        (Variables|/Game/Code/Blueprints/Widget/A_Art_Widget.A_Art_Widget_C|SetIndex _array_element _array_index))
      (:then_1
        (Variables|/Game/Code/Blueprints/Widget/A_Art_Widget.A_Art_Widget_C|SetUpdate_Period _array_element (Utilities|Array|Length _outactors)))
      (:then_2
        (bind _output_get (Variables|/Game/Code/Blueprints/Widget/A_Art_Widget.A_Art_Widget_C|SetBegin_Delay _array_element (Variables|Default|GetBegin_Delay)))
        (Variables|Default|SetBegin_Delay (+ _output_get 0.2)))
      (:then_3
        (Variables|/Game/Code/Blueprints/Widget/A_Art_Widget.A_Art_Widget_C|SetDelay_Between_Art _array_element (Math|Random|RandomFloatinRange (Variables|Default|GetDelay_Between_Art_Min) (Variables|Default|GetDelay_Between_Art_Max))))
      (:then_4
        (Default|Init _array_element)))))

(event EventBeginPlay
  (bind _returnvalue (Class|CMARTBOXDB|FonCountReq (Variables|Default|GetvUDBComp)))
  (bind _outactors (Actor|GetAllActorsOfClass "/Game/Code/Blueprints/Widget/A_Art_Widget.A_Art_Widget_C"))
  (for (_array_element _array_index) _outactors
    (Utilities|FlowControl|Sequence
      (:then_0
        (Variables|/Game/Code/Blueprints/Widget/A_Art_Widget.A_Art_Widget_C|SetIndex _array_element _array_index))
      (:then_1
        (Variables|/Game/Code/Blueprints/Widget/A_Art_Widget.A_Art_Widget_C|SetUpdate_Period _array_element (Utilities|Array|Length _outactors)))
      (:then_2
        (bind _output_get (Variables|/Game/Code/Blueprints/Widget/A_Art_Widget.A_Art_Widget_C|SetBegin_Delay _array_element (Variables|Default|GetBegin_Delay)))
        (Variables|Default|SetBegin_Delay (+ _output_get 0.2)))
      (:then_3
        (Variables|/Game/Code/Blueprints/Widget/A_Art_Widget.A_Art_Widget_C|SetDelay_Between_Art _array_element (Math|Random|RandomFloatinRange (Variables|Default|GetDelay_Between_Art_Min) (Variables|Default|GetDelay_Between_Art_Max))))
      (:then_4
        (Default|Init _array_element)))))

(event EventTick
  (params (DeltaSeconds :type Float%20%28single-precision%29)))

(fn ConstructionScript)